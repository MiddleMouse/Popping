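; Balloon on a string that floats upward and can be tied to a component at a given location.
; BeginPlay randomises the string length and applies it as the physics constraint's linear Z limit.
; AttachComponent constrains the balloon to the target component and pins the visual cable's end at that spot in the component's local space.
; Tick pushes upward at a point above the balloon's location, applying the uplift force.
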(event Custom|AttachComponent
  (params (AttachedComponent :type Primitive%20Component%20Object%20Reference) (AttachBoneName :type Name) (AttachLocation :type Vector))
  (bind _cable (Variables|Default|GetCable))
  ;[1 1 1] attach balloon at location
  (Class|PhysicsConstraintComponent|SetConstrainedComponents (Variables|Default|GetPhysicsConstraint) AttachedComponent AttachBoneName (Variables|Default|GetBalloon) "None")
  (Class|CableComponent|SetAttachEndtoComponent _cable AttachedComponent "None")
  (Variables|/Script/CableComponent.CableComponent|SetEndLocation _cable (Math|Transform|InverseTransformLocation (Transformation|GetWorldTransform AttachedComponent) AttachLocation)))

(event EventBeginPlay
  ;[1 1 1] Random string length +-15
  (Variables|Default|SetStringLength (+ (Variables|Default|GetStringLength) (Math|Random|RandomFloatinRange -15.0 15.0)))
  (Class|PhysicsConstraintComponent|SetLinearZLimit (Variables|Default|GetPhysicsConstraint) "LCM_Limited" (Variables|Default|GetStringLength)))

(event EventTick
  (params (DeltaSeconds :type Float%20%28single-precision%29))
  ;[1 1 1] floating upwards every tick
  (Class|PrimitiveComponent|AddForceatLocation (Variables|Default|GetBalloon) (Math|Vector|MakeVector 0.0 0.0 (Variables|Default|GetUpliftForce)) (+ (Transformation|GetWorldLocation (Variables|Default|GetBalloon)) "0.000000,0.000000,50.000000") "None"))

(fn ConstructionScript)