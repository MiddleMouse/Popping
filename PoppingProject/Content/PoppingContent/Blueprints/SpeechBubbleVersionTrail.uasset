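; Speech bubble balloon actor that floats upward on a tether and displays a configurable string on two text renders.
; The construction script applies the selected balloon mesh, and BeginPlay fills in the text.
; An attach event links the balloon to a given component with a physics constraint and pins the cable end at the supplied location.
; Tick applies upward force slightly above the balloon's origin to keep it afloat.
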(event Custom|AttachComponent
  (params (AttachedComponent :type Primitive%20Component%20Object%20Reference) (AttachBoneName :type Name) (AttachLocation :type Vector))
  (bind _cable (Variables|Default|GetCable))
  ;[1 1 1] attach balloon at location
  (Class|PhysicsConstraintComponent|SetConstrainedComponents (Variables|Default|GetPhysicsConstraint) AttachedComponent AttachBoneName (Variables|Default|GetSpeechBalloonTrail) "None")
  (Class|CableComponent|SetAttachEndtoComponent _cable AttachedComponent "None")
  (Variables|/Script/CableComponent.CableComponent|SetEndLocation _cable (Math|Transform|InverseTransformLocation (Transformation|GetWorldTransform AttachedComponent) AttachLocation)))

(event EventBeginPlay
  (bind _textrender (Variables|Default|GetTextRender))
  (bind _textstring (Variables|Default|Gettextstring))
  (Rendering|Components|TextRender|SetText _textrender _textstring)
  (Rendering|Components|TextRender|SetText _textrender _textstring))

(event EventTick
  (params (DeltaSeconds :type Float%20%28single-precision%29))
  ;[1 1 1] floating upwards every tick
  (Class|PrimitiveComponent|AddForceatLocation (Variables|Default|GetSpeechBalloonTrail) (Math|Vector|MakeVector 0.0 0.0 2.5e+02) (+ (Transformation|GetWorldLocation (Variables|Default|GetSpeechBalloonTrail)) "0.000000,0.000000,50.000000") "None"))

(fn ConstructionScript
  (Components|StaticMesh|SetStaticMesh (Variables|Default|GetSpeechBalloonTrail) (Variables|Default|GetTypeOfSpeechBalloon)))